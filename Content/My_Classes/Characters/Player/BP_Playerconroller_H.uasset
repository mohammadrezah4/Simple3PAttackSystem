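; Player controller that handles movement and mouse-look input and switches the player's camera between shoulder and center views.
; BeginPlay caches two camera modifiers from the camera manager and the player character, then applies the shoulder view.
; ChangeCamera re-enters the same FlipFlop, alternating which modifier is enabled and calling the character's matching spring-arm function.
; Move axes are only stored in variables, while mouse axes feed pitch and yaw directly.
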(event `self.ReceiveBeginPlay`
  (bind _returnvalue (`GameplayStatics.GetPlayerCameraManager` 0))
  (`|ExecutionSequence`
    (:`then_0`
      ;[0.2837 1 0.4135] Get Camera Modifier and Make Instance
      (bind _returnvalue_2 (`PlayerCameraManager.FindCameraModifierByClass` _returnvalue "/Game/My_Classes/Characters/Player/Camera/CM_CameraModifireOne_H.CM_CameraModifireOne_H_C"))
      (set `self.ModifreOne` _returnvalue_2)
      (bind _returnvalue_3 (`PlayerCameraManager.FindCameraModifierByClass` _returnvalue "/Game/My_Classes/Characters/Player/Camera/CM_CameraModifireTwo_H.CM_CameraModifireTwo_H_C"))
      (set `self.ModifreTwo` _returnvalue_3))
    (:`then_1`
      ;[0.1874 1 0.2705] GetPlayer Character
      (bind _asbp_player_character_h (cast `/Game/My_Classes/Characters/Player/BP_PlayerCharacter_H` (`GameplayStatics.GetPlayerCharacter` 0)))
      (set `self.PlayerCharacter` _asbp_player_character_h))
    (:`then_2`
      ;[0.1199 0.1137 1] Switch camera and modifire
      (`/Engine/EditorBlueprintResources/StandardMacros.FlipFlop` :!label _label
        (:`A`
          (if (`CameraModifier.IsDisabled` (`self.ModifreTwo`))
            (`CameraModifier.EnableModifier` (`self.ModifreOne`))
            (else
              (`CameraModifier.DisableModifier` (`self.ModifreTwo`) true)
              (`CameraModifier.EnableModifier` (`self.ModifreOne`))))
          (`/Game/My_Classes/Characters/Player/BP_PlayerCharacter_H.Spring Arm Shoulder` (`self.PlayerCharacter`)))
        (:`B`
          (if (`CameraModifier.IsDisabled` (`self.ModifreOne`))
            (`CameraModifier.EnableModifier` (`self.ModifreTwo`))
            (else
              (`CameraModifier.DisableModifier` (`self.ModifreOne`) true)
              (`CameraModifier.EnableModifier` (`self.ModifreTwo`))))
          (`/Game/My_Classes/Characters/Player/BP_PlayerCharacter_H.Spring Arm Center` (`self.PlayerCharacter`)))))))

(event `InputAction|ChangeCamera`
  (params (Key :type "Key Structure"))
  ;[0.1199 0.1137 1] Switch camera and modifire
  (:`Pressed`
    (goto _label)))

(event `InputAxis|Move Forward / Backward`
  (params (AxisValue :type "Float (single-precision)"))
  ;[1 0.3765 0.3765] Movement : Get Movement Input
  (set `self.MoveFoward` AxisValue))

(event `InputAxis|Move Right / Left`
  (params (AxisValue :type "Float (single-precision)"))
  ;[1 0.3765 0.3765] Movement : Get Movement Input
  (set `self.MoveRight` AxisValue))

(event `InputAxis|Look Up / Down Mouse`
  (params (AxisValue :type "Float (single-precision)"))
  ;[1 0.3765 0.3765] Mouse Input: Get Mouse input and add it
  (`self.AddPitchInput` AxisValue))

(event `InputAxis|Turn Right / Left Mouse`
  (params (AxisValue :type "Float (single-precision)"))
  ;[1 0.3765 0.3765] Mouse Input: Get Mouse input and add it
  (`self.AddYawInput` AxisValue))

(fn `UserConstructionScript`)