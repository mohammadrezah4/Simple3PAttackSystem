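; Enemy character Blueprint that fights the player with an attached axe and dies when its health runs out.
; Attack faces the player and plays one of three montages chosen by the data asset from AI distance, with montage notifies starting and ending the axe's attack via interface messages.
; Incoming hits ignore Enemy-tagged attackers, update the health widget, play a directional hit or death montage, then destroy the actor on death.
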(event `self.ReceiveBeginPlay`
  (`|ExecutionSequence`
    (:`then_0`
      ;[0.8612 0.1332 1] get helath widget
      (bind _asui_enemy_widget_h (cast `/Game/My_Classes/GameFile/UI_EnemyWidget_H` (`WidgetComponent.GetWidget` (`self.HealthWidget`))))
      (bind _output_get (set `self.Enemy Widget Health` _asui_enemy_widget_h))
      (set `/Game/My_Classes/GameFile/UI_EnemyWidget_H.Health` 100.0 _output_get))
    (:`then_1`
      ;[0.5184 0.3176 1] Attach Weapn to Character
      (bind _returnvalue (`|SpawnActorFromClass` "/Game/My_Classes/Weapon/AC_WaeponActor_H.AC_WaeponActor_H_C" (`self.GetTransform`) "AlwaysSpawn" "OverrideRootScale" null null))
      (bind _output_get_2 (set `self.AXE_Weapon` _returnvalue))
      (`self.K2_AttachToComponent` _output_get_2 (`self.Mesh`) "AXE_Socket" "SnapToTarget" "SnapToTarget" "KeepRelative" true))))

(event `First Attack`
  (bind _axe_weapon (`self.AXE_Weapon`))
  ;[0 0.0615 1] Attack Montage  Events (Run Combo Montage)
  (`|PlayMontage` (`self.Mesh`) "/Game/My_Classes/Characters/Player/Animation/AM_Attack01_H.AM_Attack01_H"
    (:`OnNotifyBegin`
      (message `/Game/My_Classes/Weapon/BI_Attack_InterFace_H.BI_StartAttack` _axe_weapon false self))
    (:`OnNotifyEnd`
      (message `/Game/My_Classes/Weapon/BI_Attack_InterFace_H.BI_EndAttack` _axe_weapon))))

(event `Attack`
  ;[0.2557 0.9203 1] Call Attack Randomly
  (bind _attacknumber (`/Game/My_Classes/Characters/PDA_AIDataAsstBlueprint_H.ChooseAttackAnimation` (`self.EnemyDataAsset`) (`self.AICurrentDistance`)))
  (`self.K2_SetActorRotation` (`KismetMathLibrary.FindLookAtRotation` (`SceneComponent.K2_GetComponentLocation` (`self.Mesh`)) (`SceneComponent.K2_GetComponentLocation` (`Character.Mesh` (`GameplayStatics.GetPlayerCharacter` 0)))))
  (switch `int` _attacknumber
    (:`0`
      (`self.First Attack`))
    (:`1`
      (`self.Second Attak`))
    (:`2`
      (`self.Third Attak`))))

(event `Second Attak`
  (bind _axe_weapon (`self.AXE_Weapon`))
  ;[0 0.0615 1] Attack Montage  Events (Run Combo Montage)
  (`|PlayMontage` (`self.Mesh`) "/Game/My_Classes/Characters/Player/Animation/AM_Attack02_H.AM_Attack02_H"
    (:`OnNotifyBegin`
      (message `/Game/My_Classes/Weapon/BI_Attack_InterFace_H.BI_StartAttack` _axe_weapon true self))
    (:`OnNotifyEnd`
      (message `/Game/My_Classes/Weapon/BI_Attack_InterFace_H.BI_EndAttack` _axe_weapon))))

(event `/Game/My_Classes/Weapon/BI_Attack_InterFace_H.BI_HitData`
  (params (HitLocation :type Name) (Attacker :type "Actor Object Reference") (`Attack Damage` :type "Float (double-precision)") (AttackDirection :type Integer))
  ;[1 0.1442 0.194] ApplyDamage
  (if (not (`self.ActorHasTag` Attacker "Enemy"))
    (bind _is_dead_ (`self.Calculat and set health` `Attack Damage`))
    ;;[1 0.7352 0.1944] Select Hit And Death Aniamtion
    (`|PlayMontage` (`self.Mesh`) (select `bool` _is_dead_ :`false` (select `int` AttackDirection :`0` "/Game/My_Classes/Characters/Enemy/Animation/AM_LeftHit_H.AM_LeftHit_H" :`1` "/Game/My_Classes/Characters/Enemy/Animation/AM_RightHit_H.AM_RightHit_H" :`2` "/Game/My_Classes/Characters/Enemy/Animation/AM_RightHit_H.AM_RightHit_H" :`3` "/Game/My_Classes/Characters/Enemy/Animation/AM_FrontHit_H.AM_FrontHit_H" :`4` "/Game/My_Classes/Characters/Enemy/Animation/AM_FrontHit_H.AM_FrontHit_H" :`5` "/Game/My_Classes/Characters/Enemy/Animation/AM_BackHit_H.AM_BackHit_H" :`6` "/Game/My_Classes/Characters/Enemy/Animation/AM_BackHit_H.AM_BackHit_H" :`7` "/Game/My_Classes/Characters/Enemy/Animation/AM_LeftHit_H.AM_LeftHit_H" :!type "AnimMontage Object Reference") :`true` (select `int` AttackDirection :`0` "/Game/My_Classes/Characters/Enemy/Animation/AM_SideDeath.AM_SideDeath" :`1` "/Game/My_Classes/Characters/Enemy/Animation/AM_SideDeath.AM_SideDeath" :`2` "/Game/My_Classes/Characters/Enemy/Animation/AM_SideDeath.AM_SideDeath" :`3` "/Game/My_Classes/Characters/Enemy/Animation/AM_FrontDeath_H.AM_FrontDeath_H" :`4` "/Game/My_Classes/Characters/Enemy/Animation/AM_FrontDeath_H.AM_FrontDeath_H" :`5` "/Game/My_Classes/Characters/Enemy/Animation/AM_BackDeath_H.AM_BackDeath_H" :`6` "/Game/My_Classes/Characters/Enemy/Animation/AM_BackDeath_H.AM_BackDeath_H" :`7` "/Game/My_Classes/Characters/Enemy/Animation/AM_SideDeath.AM_SideDeath" :!type "AnimMontage Object Reference"))
      (:`then`
        ;;[1 0.3209 0.788] Destroy After Death
        (if _is_dead_
          (`self.DetachFromControllerPendingDestroy`)
          (`KismetSystemLibrary.Delay` 1.5)
          (`self.K2_DestroyActor`))))))

(event `Third Attak`
  (bind _axe_weapon (`self.AXE_Weapon`))
  ;[0 0.0615 1] Attack Montage  Events (Run Combo Montage)
  (`|PlayMontage` (`self.Mesh`) "/Game/My_Classes/Characters/Player/Animation/AM_Attack03_H.AM_Attack03_H"
    (:`OnNotifyBegin`
      (message `/Game/My_Classes/Weapon/BI_Attack_InterFace_H.BI_StartAttack` _axe_weapon true self))
    (:`OnNotifyEnd`
      (message `/Game/My_Classes/Weapon/BI_Attack_InterFace_H.BI_EndAttack` _axe_weapon))))

(fn `UserConstructionScript`)