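; Axe weapon actor that detects melee hits during an attack and reports them to the struck actor.
; Attack start and end interface events start and clear a fast looping timer that sphere-traces between the blade's top and bottom points.
; Hits on attack-interface actors send bone name, attacker, fixed damage and a yaw-based quarter-turn direction, throttled by a DoOnce with delayed reset.
; It also tracks a chained-attack count on the same target.
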(event `/Game/My_Classes/Weapon/BI_Attack_InterFace_H.BI_StartAttack`
  (params (Chained :type Boolean) (Owner :type "Actor Object Reference"))
  ;[0.3326 0.1499 1] Calaculate Hit by Sphere Trace
  ;;[1 0.1669 0.8269] Draw Sphere Trace In the Start Attack
  (set `self.OwnerActor` Owner)
  (set `self.Chained` Chained)
  (bind _returnvalue (`KismetSystemLibrary.K2_SetTimerDelegate` (delegate `TraceLoop`) 0.001 true))
  (set `self.AXE_Trace_Loop` _returnvalue))

(event `TraceLoop`
  ;[0.3326 0.1499 1] Calaculate Hit by Sphere Trace
  ;;[1 0.1669 0.8269] Draw Sphere Trace In the Start Attack
  (bind (_outhit _returnvalue) (`KismetSystemLibrary.SphereTraceSingle` (`SceneComponent.K2_GetComponentLocation` (`self.AXE_Top_Point`)) (`SceneComponent.K2_GetComponentLocation` (`self.AXE_Down_Point`)) 10.0 "TraceTypeQuery2"))
  (if _returnvalue
    (bind (_bblockinghit _binitialoverlap _time _distance _location _impactpoint _normal _impactnormal _physmat _hitactor _hitcomponent _hitbonename) (`GameplayStatics.BreakHitResult` _outhit))
    (if (`KismetSystemLibrary.DoesImplementInterface` _hitactor "/Game/My_Classes/Weapon/BI_Attack_InterFace_H.BI_Attack_InterFace_H_C")
      (bind _output_get (set `self.Hitted_Actor_Not_Changed` (== (`self.Hit Actor`) _hitactor)))
      (if (not _output_get)
        (set `self.Hit Actor` _hitactor)
        (set `self.AttackNumber` 1))
      (`/Engine/EditorBlueprintResources/StandardMacros.DoOnce` false :!label _label
        (:`Completed`
          (set `self.HitLocation` _hitbonename)
          (bind (_returnvalue_roll _returnvalue_pitch _returnvalue_yaw) (`KismetMathLibrary.BreakRotator` (`KismetMathLibrary.FindLookAtRotation` (`self.K2_GetActorLocation` _hitactor) (`self.K2_GetActorLocation` (`self.OwnerActor`)))))
          (bind (_returnvalue_roll_2 _returnvalue_pitch_2 _returnvalue_yaw_2) (`KismetMathLibrary.BreakRotator` (`self.K2_GetActorRotation` _hitactor)))
          (bind _returnvalue_2 (`KismetMathLibrary.Round` (/ (- (`self.Make Degree 0-360` _returnvalue_yaw) (`self.Make Degree 0-360` _returnvalue_yaw_2)) 90.0)))
          (set `self.Direction` (`KismetMathLibrary.SelectInt` _returnvalue_2 (+ _returnvalue_2 7) (> _returnvalue_2 0)))
          (if (and (`self.Chained`) (`self.Hitted_Actor_Not_Changed`))
            (`/Engine/EditorBlueprintResources/StandardMacros.IncrementInt` (`self.AttackNumber`)
              (:`  `
                _))
            (else
              (set `self.AttackNumber` 1)))
          (message `/Game/My_Classes/Weapon/BI_Attack_InterFace_H.BI_HitData` (`self.Hit Actor`) (`self.HitLocation`) (`self.OwnerActor`) 10.0 (`self.Direction`))
          (`KismetSystemLibrary.Delay` 0.5)
          (goto _label :!via `Reset`))))))

(event `/Game/My_Classes/Weapon/BI_Attack_InterFace_H.BI_EndAttack`
  ;[0.3326 0.1499 1] Calaculate Hit by Sphere Trace
  ;;[1 0.1248 0.8799] Stop Draw Sphere Trace In the End Attack
  (`KismetSystemLibrary.K2_ClearAndInvalidateTimerHandle` (`self.AXE_Trace_Loop`)))

(fn `EndAttack`
  (returns (Hit :type Boolean))
  (return false))

(fn `UserConstructionScript`)